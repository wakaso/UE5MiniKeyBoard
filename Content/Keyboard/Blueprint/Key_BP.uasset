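; Key_BP is a single interactive keyboard key that moves down, plays a sound and changes its keycap look.
; Current and next key presets supply the logo texture, color and sound (Cue or Wave) to a dynamic material and audio component.
; Timelines drive hover and press travel, with mouse presses starting from the hover depth.
; The first release after each ResetKey swaps to the next logo and blends to its color.
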(event Custom|SetNextKeySkin
  (bind _keydym (Variables|Default|GetKeyDYM))
  (bind _nextkeyset (Variables|Default|GetNextKeySet))
  ;[1 1 1] 键帽切换颜色与图案
  (Rendering|Material|SetTextureParameterValue _keydym "LOGO" (.pic _nextkeyset))
  (bind _color (Timeline|ChangeC Play)
    (:Update
      (Rendering|Material|SetVectorParameterValue _keydym "PrimaryColor" (Math|Color|Lerp(LinearColor) (.keycolor (Variables|Default|GetCurrentKeySet)) (.keycolor _nextkeyset) _color) :!class /Script/Engine.MaterialInstanceDynamic))))

(event EventBeginPlay
  (bind _key (Variables|Default|GetKey))
  ;[1 1 1] 开始
  (bind _returnvalue (Rendering|Material|CreateDynamicMaterialInstance _key 0 "/Game/Keyboard/Mat/M_Key.M_Key" "None" :!class /Script/Engine.PrimitiveComponent))
  (bind _output_get (Variables|Default|SetKeyDYM _returnvalue))
  (Rendering|Material|SetMaterial _key 0 _output_get))

(event EventKeyReleased
  (params (KeyIndex :type Integer) (InteractivityType :type InteractivityType_Enum%20Enum :default "NewEnumerator0"))
  ;[1 1 1] 按键释放
  (switch Utilities|FlowControl|Switch|SwitchonInteractivityType_Enum InteractivityType
    (:NewEnumerator0
      _)
    (:NewEnumerator1
      _)
    (:NewEnumerator2
      _))
  (Utilities|FlowControl|Sequence
    (:then_0
      (Utilities|FlowControl|DoOnce false
        (:Completed
          (CallFunction|SetNextKeySkin))))
    (:then_1
      ;[1 1 1] 按键按下
      (bind _mov (Timeline|Mov1 Reverse)
        (:Update
          (Transformation|SetRelativeLocation (Variables|Default|GetKey) (Math|Vector|Lerp(Vector) (Variables|Default|GetPressOffset) "0.000000,0.000000,-20.000000" _mov) false false))))))

(event EventKeyRemove
  ;[1 1 1] 鼠标划过按键
  (bind _mov (Timeline|Move2 ReverseFromEnd)
    (:Update
      (Transformation|SetRelativeLocation (Variables|Default|GetKey) (Math|Vector|Lerp(Vector) "0, 0, 0" "0.000000,0.000000,-10.000000" _mov) false false))))

(event EventKeyPressed
  (params (KeyIndex :type Integer) (InteractivityType :type InteractivityType_Enum%20Enum :default "NewEnumerator0"))
  ;[1 1 1] 按键按下
  (bind _output_get (Variables|Default|SetInteractivity%20Type InteractivityType))
  (switch Utilities|FlowControl|Switch|SwitchonInteractivityType_Enum _output_get
    (:NewEnumerator0
      (Variables|Default|SetPressOffset "0.000000,0.000000,-10.000000"))
    (:NewEnumerator1
      (Variables|Default|SetPressOffset "0, 0, 0"))
    (:NewEnumerator2
      (Variables|Default|SetPressOffset "0, 0, 0")))
  (Audio|Components|Audio|Play (Variables|Default|GetAudio) 0.0)
  (bind _mov (Timeline|Mov1 Play)
    (:Update
      (Transformation|SetRelativeLocation (Variables|Default|GetKey) (Math|Vector|Lerp(Vector) (Variables|Default|GetPressOffset) "0.000000,0.000000,-20.000000" _mov) false false))))

(event EventStartSetKey
  (params (CurrentKeySet :type Key%20Set%20Single%20Structure) (NextKeySet :type Key%20Set%20Single%20Structure))
  (bind _audio (Variables|Default|GetAudio))
  (bind _keydym (Variables|Default|GetKeyDYM))
  ;[1 1 1] 初始设置按键信息
  (Variables|Default|SetCurrentKeySet CurrentKeySet)
  (Variables|Default|SetNextKeySet NextKeySet)
  (Variables|Default|SetKeyIndex (.keyindex (Variables|Default|GetCurrentKeySet)))
  (Rendering|Material|SetTextureParameterValue _keydym "LOGO" (.pic (Variables|Default|GetCurrentKeySet)))
  (Rendering|Material|SetVectorParameterValue _keydym "PrimaryColor" (.keycolor (Variables|Default|GetCurrentKeySet)) :!class /Script/Engine.MaterialInstanceDynamic)
  (if (.isusecue (Variables|Default|GetCurrentKeySet))
    (Audio|Components|Audio|SetSound _audio (.soundcue (Variables|Default|GetCurrentKeySet)))
    (else
      (Audio|Components|Audio|SetSound _audio (.soundwave (Variables|Default|GetCurrentKeySet))))))

(event EventResetKey
  ;[1 1 1] 按键释放
  (Utilities|FlowControl|DoOnce false) ; enters at Reset
)

(event EventSetNextKey
  (params (NextKey :type Key%20Set%20Single%20Structure))
  ;[1 1 1] 设置下一轮键帽预设
  (Variables|Default|SetCurrentKeySet (Variables|Default|GetNextKeySet))
  (Variables|Default|SetNextKeySet NextKey))

(event EventKeyCovered
  (params (KeyIndex :type Integer))
  ;[1 1 1] 鼠标划过按键
  (bind _mov (Timeline|Move2 PlayFromStart)
    (:Update
      (Transformation|SetRelativeLocation (Variables|Default|GetKey) (Math|Vector|Lerp(Vector) "0, 0, 0" "0.000000,0.000000,-10.000000" _mov) false false))))

(fn ConstructionScript)

(fn CheckKeyClicked
  (return))

(fn GetNextKey
  (params (KeyIndex :type Integer))
  (return ""))
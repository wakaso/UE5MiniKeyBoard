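; Interactive keyboard actor that spawns key child actors from KeyboardSets and cycles to the next themed set once every key has been pressed.
; Timelines tilt the board per key on hover and press, with press rotation chosen by mouse or keyboard input.
; Completing a round plays a sound, recolors the board's dynamic material and BP_Env background, and re-arms a DoOnce that resets keys and preloads their following set on the next release.
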(event EventBeginPlay
  (bind _board (Variables|Default|GetBoard))
  (bind _keyboardsets (Variables|Default|GetKeyboardSets))
  (bind _output (Utilities|Array|Get(acopy) _keyboardsets 1))
  (bind _output_2 (Utilities|Array|Get(acopy) _keyboardsets))
  ;[1 1 1] 开始：设置背景，键盘颜色，键帽信息
  (bind _returnvalue (Actor|GetActorOfClass "/Game/Keyboard/Background/BP_Env.BP_Env_C"))
  (Variables|Default|SetEnv _returnvalue)
  (bind _returnvalue_2 (Rendering|Material|CreateDynamicMaterialInstance _board 0 "/Game/Keyboard/Mat/M_Keyboard.M_Keyboard" "KBInst" :!class /Script/Engine.PrimitiveComponent))
  (bind _output_get (Variables|Default|SetKeyboardDYM _returnvalue_2))
  (Rendering|Material|SetMaterial _board 0 _output_get)
  (Variables|Default|SetMaxRound (- (Utilities|Array|Length _keyboardsets) 1))
  (Variables|Default|SetRoundCount 0)
  (Rendering|Material|SetVectorParameterValue (Variables|Default|GetKeyboardDYM) "PrimaryColor" (.keyboardcolor _output_2) :!class /Script/Engine.MaterialInstanceDynamic)
  (Default|ChangeBGC (Variables|Default|GetEnv) (.bgcolor _output_2))
  (for (_array_element _array_index) (.keyset _output_2)
    (bind _returnvalue_3 (AddComponent|AddChildActorComponent false (Math|Transform|MakeTransform (Utilities|Array|Get(acopy) (Variables|Default|GetSpawnList) _array_index) "0, 0, 0" "1.000000,1.000000,1.000000")))
    (Utilities|Array|Add (Variables|Default|GetKeyActors) (Variables|/Script/Engine.ChildActorComponent|GetChildActor _returnvalue_3))
    (Class|MouseInteractionBPI|StartSetKey(Message) (Variables|/Script/Engine.ChildActorComponent|GetChildActor _returnvalue_3) (Utilities|Struct|MakeKeySetSingle (.KeyType (Utilities|Struct|BreakKeySetSingle _array_element)) (.KeyIndex (Utilities|Struct|BreakKeySetSingle _array_element)) (.Pic (Utilities|Struct|BreakKeySetSingle _array_element)) (.SoundWave (Utilities|Struct|BreakKeySetSingle _array_element)) (.IsUseCue (Utilities|Struct|BreakKeySetSingle _array_element)) (.SoundCue (Utilities|Struct|BreakKeySetSingle _array_element)) (select (.keycolorfollow _output_2) (.keyboardcolor _output_2) (.KeyColor (Utilities|Struct|BreakKeySetSingle _array_element)))) (Utilities|Struct|MakeKeySetSingle (.KeyType (Utilities|Struct|BreakKeySetSingle (Utilities|Array|Get(acopy) (.keyset _output) _array_index))) (.KeyIndex (Utilities|Struct|BreakKeySetSingle (Utilities|Array|Get(acopy) (.keyset _output) _array_index))) (.Pic (Utilities|Struct|BreakKeySetSingle (Utilities|Array|Get(acopy) (.keyset _output) _array_index))) (.SoundWave (Utilities|Struct|BreakKeySetSingle (Utilities|Array|Get(acopy) (.keyset _output) _array_index))) (.IsUseCue (Utilities|Struct|BreakKeySetSingle (Utilities|Array|Get(acopy) (.keyset _output) _array_index))) (.SoundCue (Utilities|Struct|BreakKeySetSingle (Utilities|Array|Get(acopy) (.keyset _output) _array_index))) (select (.keycolorfollow _output) (.keyboardcolor _output) (.KeyColor (Utilities|Struct|BreakKeySetSingle (Utilities|Array|Get(acopy) (.keyset _output) _array_index))))))))

(event EventKeyPressed
  (params (KeyIndex :type Integer) (InteractivityType :type InteractivityType_Enum%20Enum :default "NewEnumerator0"))
  (bind _clickedkeys (Variables|Default|GetClickedKeys))
  ;[1 1 1] 触摸或按下棋盘反馈动画
  (switch Utilities|FlowControl|Switch|SwitchonInteractivityType_Enum InteractivityType
    (:NewEnumerator0
      (Variables|Default|SetRotate_Temp (Variables|Default|GetPassRotate)))
    (:NewEnumerator2
      (Variables|Default|SetRotate_Temp (Variables|Default|GetPressRotate))))
  (if (Utilities|Array|Get(acopy) _clickedkeys KeyIndex)
    _
    (else
      (Utilities|Array|SetArrayElem _clickedkeys KeyIndex true)))
  (Class|MouseInteractionBPI|KeyPressed(Message) (Utilities|Array|Get(acopy) (Variables|Default|GetKeyActors) KeyIndex) KeyIndex "NewEnumerator2")
  (bind _mov (Timeline|Mov1 PlayFromStart)
    (:Update
      (Transformation|SetActorRotation (Math|Rotator|Lerp(Rotator) "0.000000,-45.000000,0.000000" (Utilities|Array|Get(acopy) (Variables|Default|GetRotate_Temp) KeyIndex) _mov) true))))

(event EventKeyReleased
  (params (KeyIndex :type Integer) (InteractivityType :type InteractivityType_Enum%20Enum :default "NewEnumerator0"))
  ;[1 1 1] 释放按钮反馈动画
  (Utilities|FlowControl|Sequence
    (:then_0
      (Utilities|FlowControl|DoOnce true :!label _label
        (:Completed
          (for (_array_element _array_index) (Variables|Default|GetKeyActors)
            (Class|MouseInteractionBPI|ResetKey(Message) _array_element)
            (bind _nextkeys (CallFunction|GetNextKey _array_index))
            (Class|MouseInteractionBPI|SetNextKey(Message) _array_element _nextkeys)))))
    (:then_1
      (Class|MouseInteractionBPI|KeyReleased(Message) (Utilities|Array|Get(acopy) (Variables|Default|GetKeyActors) KeyIndex) KeyIndex InteractivityType)
      (if (not (Utilities|Array|ContainsItem (Variables|Default|GetClickedKeys) false))
        (Audio|PlaySound2D "/Game/Keyboard/Sound/Wave/Sound24.Sound24" 1.0 1.0 0.0 0 0)
        (Utilities|FlowControl|Sequence
          (:then_0
            (Rendering|Material|SetVectorParameterValue (Variables|Default|GetKeyboardDYM) "PrimaryColor" (.keyboardcolor (Utilities|Array|Get(acopy) (Variables|Default|GetKeyboardSets) (+ (Variables|Default|GetRoundCount) 1))) :!class /Script/Engine.MaterialInstanceDynamic)
            (Default|ChangeBGC (Variables|Default|GetEnv) (.bgcolor (Utilities|Array|Get(acopy) (Variables|Default|GetKeyboardSets) (+ (Variables|Default|GetRoundCount) 1))))
            (bind _result (Math|Integer|IncrementInt (Variables|Default|GetRoundCount))
              (:%20%20
                (if (== _result (Variables|Default|GetMaxRound))
                  (Variables|Default|SetRoundCount 0))
                (Variables|Default|SetClickedKeys (Variables|Default|GetClickedKeys_O)))))
          (:then_1
            (goto _label Reset)))))))

(event EventKeyCovered
  (params (KeyIndex :type Integer))
  ;[1 1 1] 鼠标经过
  (Variables|Default|SetIsCovered true)
  (bind _mov (Timeline|时间轴 PlayFromStart)
    (:Update
      (Transformation|SetActorRotation (Math|Rotator|Lerp(Rotator) "0.000000,-45.000000,0.000000" (Utilities|Array|Get(acopy) (Variables|Default|GetPassRotate) KeyIndex) _mov) true))))

(event EventKeyRemove
  ;[1 1 1] 鼠标经过
  (Variables|Default|SetIsCovered false)
  (bind _mov (Timeline|时间轴 Reverse)
    (:Update
      (Transformation|SetActorRotation (Math|Rotator|Lerp(Rotator) "0.000000,-45.000000,0.000000" (Utilities|Array|Get(acopy) (Variables|Default|GetPassRotate) (stale EventKeyCovered KeyIndex)) _mov) true))))

(fn ConstructionScript)

(fn CheckKeyClicked
  (return))

(fn GetNextKey
  (params (KeyIndex :type Integer))
  (bind _roundcount (Variables|Default|GetRoundCount))
  (bind _keyboardsets (Variables|Default|GetKeyboardSets))
  (bind _returnvalue (+ _roundcount 1))
  (bind _output (Utilities|Array|Get(acopy) _keyboardsets _returnvalue))
  (bind _output_2 (Utilities|Array|Get(acopy) (.keyset _output) KeyIndex))
  (bind (_keytype _keyindex _pic _soundwave _isusecue _soundcue _keycolor) (Utilities|Struct|BreakKeySetSingle _output_2))
  (return (Utilities|Struct|MakeKeySetSingle _keytype _keyindex _pic _soundwave _isusecue _soundcue (select (.keycolorfollow _output) (.keyboardcolor _output) _keycolor))))

(fn ResetKey
  (return))